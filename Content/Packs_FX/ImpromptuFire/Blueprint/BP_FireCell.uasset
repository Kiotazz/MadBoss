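; One cell of a grid-based spreading fire, igniting when fire damage depletes its HP.
; Ignition places particles, sound and fading scorch decals at a surface found by six axis traces.
; While alight, its Tick periodically damages nearby BP_FireInterface actors, using wind direction and random intervals to vary spread.
; Settings volumes can override tuning, auto-ignite or block it; cells burn out, reset, or get culled and removed from their grid.
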(event Custom|UpdateNearbyBurnables
  ;[1 1 1] Get surrounding burnable actors
  (bind _outactors (Collision|SphereOverlapActors (Transformation|GetActorLocation) (* (Variables|Default|GetCellHalfSize) (Variables|Default|GetRadiusToAffectActors)) (Utilities|Array|MakeArray "ObjectTypeQuery2" "ObjectTypeQuery1" "ObjectTypeQuery4") "/Script/Engine.Actor")) ; get nearby objects to damage.
  (Utilities|Array|Clear (Variables|Default|GetNearbyBurnableActors))
  (for _array_element _outactors
    (if (and (Utilities|IsValid _array_element) (Utilities|DoesObjectImplementInterface _array_element "/Game/Packs_FX/ImpromptuFire/Blueprint/BP_FireInterface.BP_FireInterface_C"))
      (Utilities|Array|Add (Variables|Default|GetNearbyBurnableActors) _array_element))))

(event Custom|ResetCell
  ;[1 1 1] Reset the cell so it can be ignited again
  ;[1 1 1] Response to burn damage inflicted upon this actor
  (Variables|FireSpreading|SetHP (Variables|Default|GetInitialHP))
  (Utilities|FlowControl|DoOnce false) ; enters at Reset
)

(event Custom|MakeScorchDecals
  (bind _returnvalue (Math|Random|RandomFloatinRange 0.8 2.2))
  (bind _cellhalfsize (Variables|Default|GetCellHalfSize))
  (bind _decalsizescalar (Variables|Decals|GetDecalSizeScalar))
  (bind _nearestsurfacenormal (Variables|Default|GetNearestSurfaceNormal))
  (bind _returnvalue_2 (Math|Conversions|RotationFromXVector _nearestsurfacenormal))
  (bind _returnvalue_3 (* _cellhalfsize _decalsizescalar))
  (bind (_roll _pitch _yaw) (Math|Rotator|BreakRotator _returnvalue_2))
  (bind _returnvalue_4 (* _returnvalue_3 _returnvalue))
  ;[1 1 1] Make scorch decals on nearest surface - fade them in, fade out red glow, fade out opacity, kill cell on fully faded out. Adjust timeline FadeDecal to change fade timing
  (if (Variables|/Game/Packs_FX/ImpromptuFire/Blueprint/BP_ImpromptuFireGrid.BP_ImpromptuFireGrid_C|GetMakeScorchDecals (Variables|Default|GetOwningGrid))
    (bind _returnvalue_5 (Rendering|Decal|SpawnDecalatLocation (Variables|Decals|GetScorchDecalMaterial) (Math|Vector|MakeVector _returnvalue_4 _returnvalue_4 (Variables|Decals|GetDecalDepth)) (Variables|Default|GetNearest%20Surface%20Location) _returnvalue_2 (Variables|Decals|GetBurnDecalLifespan)))
    (Transformation|SetRelativeRotation _returnvalue_5 (Math|Rotator|MakeRotator (Math|Random|RandomFloatinRange 0.0 275.0) _pitch _yaw) false false)
    (Utilities|Array|Add (Variables|Decals|GetSpawnedDecals) _returnvalue_5) ; Having decals in an array helps them not get aggressively culled by the engine
    (bind _returnvalue_6 (Rendering|Material|CreateDynamicMaterialInstance "/Game/Packs_FX/ImpromptuFire/ScorchDecal/M_ScorchDecalMaterial.M_ScorchDecalMaterial" "None" "None" :!class /Script/Engine.KismetMaterialLibrary))
    (Rendering|Components|Decal|SetDecalMaterial _returnvalue_5 _returnvalue_6)
    (bind (_direction _opacity _emissive) (Timeline|FadeDecal PlayFromStart)
      (:Update
        (Rendering|Material|SetScalarParameterValue _returnvalue_6 "Opacity" _opacity :!class /Script/Engine.MaterialInstanceDynamic)
        (Rendering|Material|SetScalarParameterValue _returnvalue_6 "EmissiveAmount" _emissive :!class /Script/Engine.MaterialInstanceDynamic))
      (:Finished
        (CallFunction|DestroyCell)))))

(event Custom|CullTimer
  (bind _owninggrid (Variables|Default|GetOwningGrid))
  (bind _cellidlelifetime (Variables|Default|GetCellIdleLifetime))
  ;[1 1 1] Cull any cells which hang around un-ignited for too long
  (Variables|Default|SetInitialHP (Variables|FireSpreading|GetHP)) ; Remember our initial HP in case the cell needs to reset later
  (if (Utilities|IsValid _owninggrid)
    (if (Variables|/Game/Packs_FX/ImpromptuFire/Blueprint/BP_ImpromptuFireGrid.BP_ImpromptuFireGrid_C|GetAllowCellCull _owninggrid)
      (Utilities|FlowControl|Delay _cellidlelifetime) ; Wait a bit, then destroy self if grid was never lit.
      (if (not (Variables|FireSpreading|GetAlight))
        (if (Variables|/Game/Packs_FX/ImpromptuFire/Blueprint/BP_ImpromptuFireGrid.BP_ImpromptuFireGrid_C|GetHasBeenAlight _owninggrid)
          (Utilities|FlowControl|Delay (* _cellidlelifetime 0.5)) ; Grid was lit at some point. Wait a bit longer for this cell to catch before culling it
        )
        (if (not (Variables|FireSpreading|GetAlight))
          (CallFunction|DestroyCell))))))

(event Custom|DestroyCell
  (bind _owninggrid (Variables|Default|GetOwningGrid))
  (bind _cells (Variables|/Game/Packs_FX/ImpromptuFire/Blueprint/BP_ImpromptuFireGrid.BP_ImpromptuFireGrid_C|GetCells _owninggrid))
  ;[1 1 1] Remove cell from grid and destroy it
  (Utilities|Array|RemoveIndex _cells (Variables|Default|GetIndexOnOwningGrid))
  (if (== (Utilities|Array|LastIndex _cells) -1) ; Destroy grid actor if this cell's destruction would leave it empty
    (Default|DestroyGrid _owninggrid))
  (Actor|DestroyActor) ; Destroy this cell
)

(event EventFireDamage
  (params (Amount :type Integer))
  ;[1 1 1] Response to burn damage inflicted upon this actor
  (Variables|/Game/Packs_FX/ImpromptuFire/Blueprint/BP_ImpromptuFireGrid.BP_ImpromptuFireGrid_C|SetHasBeenAlight (Variables|Default|GetOwningGrid) true)
  (if (<= (- (Variables|FireSpreading|GetHP) Amount) 0)
    (Variables|FireSpreading|SetHP 0)
    (Utilities|FlowControl|DoOnce false ; You can only ignite once
      (:Completed
        (CallFunction|Ignite)))
    (else
      (Variables|FireSpreading|SetHP (- (Variables|FireSpreading|GetHP) Amount)))))

(event EventIgnite
  (bind _returnvalue (Math|Random|RandomFloatinRange 0.1 2.0))
  (bind _cellhalfsize (Variables|Default|GetCellHalfSize))
  (bind _returnvalue_2 (Math|Float|Clamp(Float) _returnvalue 0.5 1.75))
  (bind _returnvalue_3 (* _cellhalfsize 0.025))
  (bind _returnvalue_4 (* _returnvalue_3 _returnvalue_2))
  ;[1 1 1] Ignition
  (Actor|Tick|SetActorTickEnabled true)
  (Variables|Default|SetWind (Variables|/Game/Packs_FX/ImpromptuFire/Blueprint/BP_ImpromptuFireGrid.BP_ImpromptuFireGrid_C|GetWind (Variables|Default|GetOwningGrid)))
  (Variables|FireSpreading|SetAlight true)
  (bind (_hit_normal _hitactor _hitlocation _udfblr) (CallFunction|FindNearestSurface))
  (Variables|Default|SetNearestSurfaceNormal _hit_normal)
  (Variables|Default|SetNearest%20Surface%20Location _hitlocation)
  (if (Math|Vector|Equal(Vector) _hitlocation "0, 0, 0" 0.0001)
    (bind _returnvalue_5 (Effects|SpawnEmitteratLocation "/Game/Packs_FX/ImpromptuFire/Particles/P_FireEffect.P_FireEffect" (Transformation|GetActorLocation) (Transformation|GetActorRotation (Variables|Default|GetWind)))) ; If finding nearest surface failed somehow, spawn particles at this cell
    (Variables|Default|SetFireEmitter1 _returnvalue_5)
    (else
      (bind _returnvalue_6 (Effects|SpawnEmitteratLocation (Variables|Particles|GetFireParticle) _hitlocation (Transformation|GetActorRotation (Variables|Default|GetWind))))
      (Variables|Default|SetFireEmitter1 _returnvalue_6)))
  (if (== _udfblr 1)
    (bind _returnvalue_7 (Effects|SpawnEmitteratLocation (Variables|Particles|GetHorizontalSpreadParticle) _hitlocation "0, 0,0.000000"))
    (Variables|Default|SetFireEmitter2 _returnvalue_7))
  (if (<= _returnvalue_3 1.0)
    _
    (else
      (Transformation|SetRelativeScale3D (Variables|Default|GetFireEmitter1) (Math|Vector|MakeVector _returnvalue_4 _returnvalue_4 _returnvalue_4))))
  (bind _returnvalue_8 (Audio|SpawnSoundAttached (Variables|FireSpreading|GetFire%20Sound) (Variables|Default|GetFireEmitter1) "None" "0, 0, 0" "0, 0, 0" "KeepRelativeOffset" false 1.0 1.0 0.0 0 0))
  (Variables|Default|SetBurningSound _returnvalue_8)
  (Utilities|FlowControl|Sequence
    (:then_0
      (CallFunction|MakeScorchDecals))
    (:then_1
      (Utilities|FlowControl|Delay (Math|Random|RandomFloatinRange (Variables|FireSpreading|GetFireLifetimeMin) (Variables|FireSpreading|GetFireLifetimeMax)))
      (CallFunction|Unignite) ; Burn out
      (Utilities|FlowControl|Delay (Variables|FireSpreading|GetReBurnTime))
      (CallFunction|ResetCell))))

(event EventUnignite
  (bind _burningsound (Variables|Default|GetBurningSound))
  ;[1 1 1] Unignition
  (Actor|Tick|SetActorTickEnabled false)
  (Components|Activation|Deactivate (Variables|Default|GetFireEmitter1))
  (Utilities|FlowControl|Delay (Variables|Default|GetParticleFadeOutAllowance))
  (Components|DestroyComponent (Variables|Default|GetFireEmitter1))
  (Audio|Components|Audio|Stop _burningsound)
  (Components|DestroyComponent _burningsound)
  (Variables|FireSpreading|SetAlight false))

(event EventTick
  (params (DeltaSeconds :type Float%20%28single-precision%29))
  ;[1 1 1] Deal fire damage at intervals
  (if (Variables|FireSpreading|GetAlight) ; Only have anything to tick if alight
    (Utilities|FlowControl|Sequence
      (:then_0
        (Utilities|FlowControl|Delay (Math|Random|RandomFloatinRange (Variables|FireSpreading|GetDamageIntervalMin) (Variables|FireSpreading|GetDamageIntervalMax))) ; Deal damage every <interval>. Having this in a range helps the fire spread in a less uniform way
        (for _array_element (Variables|Default|GetNearbyBurnableActors) ; Iterate through nearby burnable actors and fire-damage them
          (if (Utilities|IsValid _array_element)
            (if (> (Math|Vector|DotProduct (Math|Vector|GetUnitDirection(Vector) (Transformation|GetActorLocation _array_element) (Transformation|GetActorLocation)) (Transformation|GetActorForwardVector (Variables|Default|GetWind))) 0.0) ; Burnable actor in wind direction?
              (Class|BPFireInterface|FireDamage(Message) _array_element (Variables|FireSpreading|GetDamageDealt)) ; Apply fire damage to burnable actors in range
              (else
                (Class|BPFireInterface|FireDamage(Message) _array_element (Variables|FireSpreading|GetDamageDealtDownwind)) ; Apply extra fire damage to burnable actors downwind
              )))))
      (:then_1
        (Utilities|FlowControl|Delay (Variables|FireSpreading|GetUpdateNearbyBurnablesInterval)) ; Update list of nearby actors to potentially spread to every few seconds.
        (CallFunction|UpdateNearbyBurnables)))))

(fn ConstructionScript)

(fn CreateCell
  (bind _cellhalfsize (Variables|Default|GetCellHalfSize))
  (bind _returnvalue (AddComponent|AddBoxComponent false))
  (Components|Box|SetBoxExtent _returnvalue (Math|Vector|MakeVector _cellhalfsize _cellhalfsize _cellhalfsize) true)
  (Variables|Default|SetBox _returnvalue)
  (CallFunction|InheritSettingsfromVolume)
  (CallFunction|CullTimer)
  (CallFunction|UpdateNearbyBurnables))

(fn OverlapCheck
  (params (Exclude :type Array%20of%20BP%20Fire%20Cell%20Object%20References))
  (bind _box (Variables|Default|GetBox))
  (bind _returnvalue (Transformation|GetWorldLocation _box))
  (bind _returnvalue_2 (Class|KismetSystemLibrary|BoxTraceSingleforObjects _returnvalue (- _returnvalue "0, 0,-0.100000") (Variables|/Script/Engine.BoxComponent|GetBoxExtent _box) "0, 0, 0" (Utilities|Array|MakeArray "ObjectTypeQuery1" "ObjectTypeQuery2") false Exclude "None" true))
  (if (not _returnvalue_2)
    (Actor|DestroyActor)))

(fn FindNearestSurface
  (bind _returnvalue (Transformation|GetActorLocation))
  (bind _owninggrid (Variables|Default|GetOwningGrid))
  ;[1 1 1] Do a trace up/down/left/right/front/back and return the shortest one
  (LocalVariables|SetSurfaceCheckDir (Math|Vector|MakeVector 0.0 0.0 (Variables|Default|GetCellHalfSize))) ; Up
  (for _index (range 1 6)
    (if (Utilities|IsValid _owninggrid)
      (bind (_outhit _returnvalue_2) (Collision|LineTraceForObjects _returnvalue (+ _returnvalue (* (LocalVariables|GetSurfaceCheckDir) 2.0)) (Utilities|Array|MakeArray "ObjectTypeQuery1") false (Variables|/Game/Packs_FX/ImpromptuFire/Blueprint/BP_ImpromptuFireGrid.BP_ImpromptuFireGrid_C|GetCells _owninggrid) "None"))
      (Utilities|FlowControl|Sequence
        (:then_0
          (if (== _index 1)
            (LocalVariables|SetSurfaceCheckDir (Math|Vector|MakeVector 0.0 0.0 (* (Variables|Default|GetCellHalfSize) -1.0))) ; Down
            (elif (== _index 2)
              (LocalVariables|SetSurfaceCheckDir (Math|Vector|MakeVector (Variables|Default|GetCellHalfSize) 0.0 0.0)) ; Front
              (elif (== _index 3)
                (LocalVariables|SetSurfaceCheckDir (Math|Vector|MakeVector (* (Variables|Default|GetCellHalfSize) -1.0) 0.0 0.0)) ; Back
                (elif (== _index 4)
                  (LocalVariables|SetSurfaceCheckDir (Math|Vector|MakeVector 0.0 (* (Variables|Default|GetCellHalfSize) -1.0) 0.0)) ; Left
                  (elif (== _index 5)
                    (LocalVariables|SetSurfaceCheckDir (Math|Vector|MakeVector 0.0 (Variables|Default|GetCellHalfSize) 0.0)) ; Right
                  ))))))
        (:then_1
          (if _returnvalue_2
            (Utilities|FlowControl|Sequence
              (:then_0
                (Utilities|FlowControl|DoOnce false
                  (:Completed
                    (LocalVariables|SetHitSomething true))))
              (:then_1
                (if (> (.Time (Collision|BreakHitResult _outhit)) (LocalVariables|GetLastTime))
                  (LocalVariables|SetNearestLoc (.ImpactPoint (Collision|BreakHitResult _outhit)))
                  (LocalVariables|SetNearestNormal (.ImpactNormal (Collision|BreakHitResult _outhit)))
                  (LocalVariables|SetNearestActor (.HitActor (Collision|BreakHitResult _outhit)))
                  (LocalVariables|SetDirection _index)))))))))
  (if (LocalVariables|GetHitSomething)
    (return (LocalVariables|GetNearestNormal) (LocalVariables|GetNearestActor) (LocalVariables|GetNearestLoc) (LocalVariables|GetDirection))
    (else
      (CallFunction|DestroyCell) ; If we weren't able to find any nearby surface, this cell is in an awkward position and should be destroyed
    )))

(fn InheritSettingsfromVolume
  (bind _box (Variables|Default|GetBox))
  (bind _outactors (Collision|BoxOverlapActors (Transformation|GetWorldLocation _box) (Variables|/Script/Engine.BoxComponent|GetBoxExtent _box) (Utilities|Array|MakeArray "ObjectTypeQuery2") "/Game/Packs_FX/ImpromptuFire/Blueprint/BP_FireSettingsVolume.BP_FireSettingsVolume_C" :!class /Script/Engine.KismetSystemLibrary))
  (bind _asbp_fire_settings_volume (Utilities|Casting|CastToBP_FireSettingsVolume (Utilities|Array|Get(acopy) _outactors))
    (:then
      (Variables|Default|SetSettingsVolume _asbp_fire_settings_volume)
      (Utilities|FlowControl|Sequence
        (:then_0
          (Utilities|IsValid (Variables|Default|GetSettingsVolume)
            (:Is%20Valid
              (if (Variables|/Game/Packs_FX/ImpromptuFire/Blueprint/BP_FireSettingsVolume.BP_FireSettingsVolume_C|GetPreventFires (Variables|Default|GetSettingsVolume))
                (CallFunction|DestroyCell)
                (else
                  (Utilities|FlowControl|Sequence
                    (:then_0
                      (if (== (Variables|/Game/Packs_FX/ImpromptuFire/Blueprint/BP_FireSettingsVolume.BP_FireSettingsVolume_C|GetCellHealth (Variables|Default|GetSettingsVolume)) 0)
                        _
                        (else
                          (Variables|FireSpreading|SetHP (Variables|/Game/Packs_FX/ImpromptuFire/Blueprint/BP_FireSettingsVolume.BP_FireSettingsVolume_C|GetCellHealth (Variables|Default|GetSettingsVolume))))))
                    (:then_1
                      (if (Variables|/Game/Packs_FX/ImpromptuFire/Blueprint/BP_FireSettingsVolume.BP_FireSettingsVolume_C|GetCellAutoIgnite (Variables|Default|GetSettingsVolume))
                        (CallFunction|Ignite)))
                    (:then_2
                      (if (== (Variables|/Game/Packs_FX/ImpromptuFire/Blueprint/BP_FireSettingsVolume.BP_FireSettingsVolume_C|GetCellDamageIntervalMax (Variables|Default|GetSettingsVolume)) 0.0)
                        _
                        (else
                          (Variables|FireSpreading|SetDamageIntervalMax (Variables|/Game/Packs_FX/ImpromptuFire/Blueprint/BP_FireSettingsVolume.BP_FireSettingsVolume_C|GetCellDamageIntervalMax (Variables|Default|GetSettingsVolume)))
                          (Variables|FireSpreading|SetDamageIntervalMin (Variables|/Game/Packs_FX/ImpromptuFire/Blueprint/BP_FireSettingsVolume.BP_FireSettingsVolume_C|GetCellDamageIntervalMin (Variables|Default|GetSettingsVolume))))))
                    (:then_3
                      (if (== (Variables|/Game/Packs_FX/ImpromptuFire/Blueprint/BP_FireSettingsVolume.BP_FireSettingsVolume_C|GetDamage (Variables|Default|GetSettingsVolume)) 0)
                        _
                        (else
                          (Variables|FireSpreading|SetDamageDealt (Variables|/Game/Packs_FX/ImpromptuFire/Blueprint/BP_FireSettingsVolume.BP_FireSettingsVolume_C|GetDamage (Variables|Default|GetSettingsVolume))))))
                    (:then_4
                      (if (== (Variables|/Game/Packs_FX/ImpromptuFire/Blueprint/BP_FireSettingsVolume.BP_FireSettingsVolume_C|GetDamageDownwind (Variables|Default|GetSettingsVolume)) 0)
                        _
                        (else
                          (Variables|FireSpreading|SetDamageDealtDownwind (Variables|/Game/Packs_FX/ImpromptuFire/Blueprint/BP_FireSettingsVolume.BP_FireSettingsVolume_C|GetDamageDownwind (Variables|Default|GetSettingsVolume))))))
                    (:then_5
                      (if (== (Variables|/Game/Packs_FX/ImpromptuFire/Blueprint/BP_FireSettingsVolume.BP_FireSettingsVolume_C|GetUpdateNearbyBurnablesInterval (Variables|Default|GetSettingsVolume)) 0.0)
                        _
                        (else
                          (Variables|FireSpreading|SetUpdateNearbyBurnablesInterval (Variables|/Game/Packs_FX/ImpromptuFire/Blueprint/BP_FireSettingsVolume.BP_FireSettingsVolume_C|GetUpdateNearbyBurnablesInterval (Variables|Default|GetSettingsVolume)))))))
                  (return))))
            (:Is%20Not%20Valid
              (return))))
        (:then_1
          (return))))
    (:CastFailed
      (return))))