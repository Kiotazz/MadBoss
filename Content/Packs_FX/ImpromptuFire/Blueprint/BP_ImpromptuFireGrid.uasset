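; Fire grid actor that fills a volume with BP_FireCell child actors wherever there is static surface to burn, optionally spawning a BP_Flame at its ignition point.
; Generation starts automatically or through Generate, with parameters optionally supplied via GetSettings.
; Box traces and overlaps reject empty or already occupied spots.
; The grid builds in delayed chunks, layer by layer, to spread load across ticks, and destroys itself if no cells result.
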(event Custom|DestroyGrid
  ;[1 1 1] If no cells were generated, destroy this grid
  (Actor|DestroyActor))

(event Custom|Generate
  (bind _returnvalue (Transformation|GetActorLocation))
  (bind _gridresolution (Variables|FireGridResolution/GenerationOptions|GetGridResolution))
  (bind _gridresolution_2 (Variables|FireGridResolution/GenerationOptions|GetGridResolution))
  (bind _gridloopdelay (Variables|Default|GetGridLoopDelay))
  (bind _gridresolution_3 (Variables|FireGridResolution/GenerationOptions|GetGridResolution))
  (bind _chunkfraction (Variables|FireGridResolution/GenerationOptions|GetChunkFraction))
  (bind _returnvalue_2 (* _gridresolution _gridresolution_2))
  (bind _returnvalue_3 (/ _returnvalue_2 _chunkfraction))
  (if (Variables|FireGrid|GetBuildGridUpwards)
    ;[1 1 1] Offset actor location going forward if we want to BuildGridUpwards
    (Transformation|SetActorLocation (+ (Transformation|GetActorLocation) (Math|Vector|MakeVector 0.0 0.0 (* (* (Variables|FireGridResolution/GenerationOptions|GetVerticalResolution) (* (Variables|FireGridResolution/GenerationOptions|GetCellHalfSize) 2.0)) 0.5))) false false)
    (Variables|FireGrid|SetIgnitionPoint (- (Variables|FireGrid|GetIgnitionPoint) (Math|Vector|MakeVector 0.0 0.0 (* (* (Variables|FireGridResolution/GenerationOptions|GetVerticalResolution) (* (Variables|FireGridResolution/GenerationOptions|GetCellHalfSize) 2.0)) 0.5)))))
  (Utilities|FlowControl|Delay (Variables|FireGrid|GetDelayBeforeStart))
  ;[1 1 1] Get Wind actor
  (bind _outactors (Actor|GetAllActorsOfClass "/Script/Engine.WindDirectionalSource"))
  (Variables|Default|SetWind (Utilities|Array|Get(acopy) _outactors))
  ;[1 1 1] Set first cell location
  (Variables|Default|SetCellLocVec (Transformation|GetActorLocation))
  ;[1 1 1] Auto-light the grid
  (if (Variables|FireGrid|GetLight%20Automatically) ; Auto light?
    (Game|SpawnActorfromClass "/Game/Packs_FX/ImpromptuFire/Blueprint/BP_Flame.BP_Flame_C" (Math|Transform|MakeTransform (Math|Transform|TransformLocation (Transformation|GetActorTransform) (Variables|FireGrid|GetIgnitionPoint)) "0, 0, 0" "1.000000,1.000000,1.000000") "AlwaysSpawn" 0 0 true))
  (for _index (range 1 _returnvalue_3) :!label _label ; Loop through checking spaces for viable cell placement, placing cells. Cycle back into this loop with new locations for each grid chunk. We can delay between loops even though this is a regular for loop because the delay is outside the loop.
    (Variables|Default|SetCurrentCellIndex (+ _index (* (Variables|Default|GetChunksDone) _returnvalue_3)))
    (bind _overlapped (CallFunction|OverlapCheck (- (Math|Transform|InverseTransformLocation (Transformation|GetActorTransform) (Variables|Default|GetCellLocVec)) (Math|Vector|MakeVector (- (* (* (Variables|FireGridResolution/GenerationOptions|GetGridResolution) (* (Variables|FireGridResolution/GenerationOptions|GetCellHalfSize) 2.0)) 0.5) (Variables|FireGridResolution/GenerationOptions|GetCellHalfSize)) (- (* (* (Variables|FireGridResolution/GenerationOptions|GetGridResolution) (* (Variables|FireGridResolution/GenerationOptions|GetCellHalfSize) 2.0)) 0.5) (Variables|FireGridResolution/GenerationOptions|GetCellHalfSize)) (- (* (* (Variables|FireGridResolution/GenerationOptions|GetGridResolution) (* (Variables|FireGridResolution/GenerationOptions|GetCellHalfSize) 2.0)) 0.5) (Variables|FireGridResolution/GenerationOptions|GetCellHalfSize)))) false)) ; Check whether space is valid for a cell. Only make one if so
    (if _overlapped
      (bind _overlappedcell (CallFunction|OverlapCheck (- (Math|Transform|InverseTransformLocation (Transformation|GetActorTransform) (Variables|Default|GetCellLocVec)) (Math|Vector|MakeVector (- (* (* (Variables|FireGridResolution/GenerationOptions|GetGridResolution) (* (Variables|FireGridResolution/GenerationOptions|GetCellHalfSize) 2.0)) 0.5) (Variables|FireGridResolution/GenerationOptions|GetCellHalfSize)) (- (* (* (Variables|FireGridResolution/GenerationOptions|GetGridResolution) (* (Variables|FireGridResolution/GenerationOptions|GetCellHalfSize) 2.0)) 0.5) (Variables|FireGridResolution/GenerationOptions|GetCellHalfSize)) (- (* (* (Variables|FireGridResolution/GenerationOptions|GetGridResolution) (* (Variables|FireGridResolution/GenerationOptions|GetCellHalfSize) 2.0)) 0.5) (Variables|FireGridResolution/GenerationOptions|GetCellHalfSize)))) true)) ; Overlap check again, this time checking only for existing cells (any grid)
      (if _overlappedcell
        (if (== (Math|Integer|%(Integer) (Variables|Default|GetCurrentCellIndex) (/ (* _gridresolution_3 _gridresolution_3) (Variables|FireGridResolution/GenerationOptions|GetGridResolution))) 0) :!label _label_2 ; Begin a new row?
          (Variables|Default|SetCellLocVec (Math|Vector|MakeVector (.x (Transformation|GetActorLocation)) (+ (.y (Variables|Default|GetCellLocVec)) (* (Variables|FireGridResolution/GenerationOptions|GetCellHalfSize) 2.0)) (.z (Variables|Default|GetCellLocVec))))
          (else
            (Variables|Default|SetCellLocVec (Math|Vector|MakeVector (+ (.x (Variables|Default|GetCellLocVec)) (* (Variables|FireGridResolution/GenerationOptions|GetCellHalfSize) 2.0)) (.y (Variables|Default|GetCellLocVec)) (.z (Variables|Default|GetCellLocVec))))))
        (else
          (bind _returnvalue_4 (AddComponent|AddChildActorComponent false (Math|Transform|MakeTransform (- (Math|Transform|InverseTransformLocation (Transformation|GetActorTransform) (Variables|Default|GetCellLocVec)) (Math|Vector|MakeVector (- (* (* (Variables|FireGridResolution/GenerationOptions|GetGridResolution) (* (Variables|FireGridResolution/GenerationOptions|GetCellHalfSize) 2.0)) 0.5) (Variables|FireGridResolution/GenerationOptions|GetCellHalfSize)) (- (* (* (Variables|FireGridResolution/GenerationOptions|GetGridResolution) (* (Variables|FireGridResolution/GenerationOptions|GetCellHalfSize) 2.0)) 0.5) (Variables|FireGridResolution/GenerationOptions|GetCellHalfSize)) (- (* (* (Variables|FireGridResolution/GenerationOptions|GetGridResolution) (* (Variables|FireGridResolution/GenerationOptions|GetCellHalfSize) 2.0)) 0.5) (Variables|FireGridResolution/GenerationOptions|GetCellHalfSize))))))) ; Make a fire cell
          (bind _asbp_fire_cell (Utilities|Casting|CastToBP_FireCell (Variables|/Script/Engine.ChildActorComponent|GetChildActor _returnvalue_4)))
          (bind _returnvalue_5 (Utilities|Array|Add (Variables|Default|GetCells) _asbp_fire_cell))
          (Variables|/Game/Packs_FX/ImpromptuFire/Blueprint/BP_FireCell.BP_FireCell_C|SetIndexOnOwningGrid _asbp_fire_cell _returnvalue_5)
          (Variables|/Game/Packs_FX/ImpromptuFire/Blueprint/BP_FireCell.BP_FireCell_C|SetOwningGrid _asbp_fire_cell self)
          (Variables|/Game/Packs_FX/ImpromptuFire/Blueprint/BP_FireCell.BP_FireCell_C|SetCellHalfSize _asbp_fire_cell (Variables|FireGridResolution/GenerationOptions|GetCellHalfSize))
          (Default|CreateCell _asbp_fire_cell)
          (if (Variables|FireGrid|GetGridVisible)
            (Development|SetHiddeninGame _asbp_fire_cell false false) ; Unhide cells
            (goto _label_2))))
      (else
        (goto _label_2))))
  ;[1 1 1] Cycle back into the ForLoop for each chunk of grid, after a delay (only so we don't try to build the whole grid on one tick).
  (Variables|Default|SetChunksDone (+ (Variables|Default|GetChunksDone) 1))
  (if (>= (Variables|Default|GetChunksDone) _chunkfraction)
    (Utilities|FlowControl|Delay _gridloopdelay)
    ;[1 1 1] Keep doing all of the above as long as there's vertical iterations remaining
    (Variables|Default|SetVerticalIterations (+ (Variables|Default|GetVerticalIterations) 1))
    (if (>= (Variables|Default|GetVerticalIterations) (Variables|FireGridResolution/GenerationOptions|GetVerticalResolution))
      (Variables|Default|SetGridFullyGenerated true)
      ;[1 1 1] If no cells were generated, destroy this grid
      (if (== (Utilities|Array|Length (Variables|Default|GetCells)) 0)
        (Actor|DestroyActor))
      (else
        ;[1 1 1] finished all rows for this height, increment new cell height
        (Variables|Default|SetCellLocVec (Math|Vector|MakeVector (.x _returnvalue) (.y _returnvalue) (+ (.z _returnvalue) (* (Variables|Default|GetVerticalIterations) (* (Variables|FireGridResolution/GenerationOptions|GetCellHalfSize) 2.0)))))
        (Variables|Default|SetChunksDone 0)
        (goto _label)))
    (else
      (Utilities|FlowControl|Delay _gridloopdelay)
      (goto _label))))

(event EventBeginPlay
  (bind _returnvalue (Transformation|GetActorLocation))
  (bind _gridresolution (Variables|FireGridResolution/GenerationOptions|GetGridResolution))
  (bind _gridresolution_2 (Variables|FireGridResolution/GenerationOptions|GetGridResolution))
  (bind _gridloopdelay (Variables|Default|GetGridLoopDelay))
  (bind _gridresolution_3 (Variables|FireGridResolution/GenerationOptions|GetGridResolution))
  (bind _chunkfraction (Variables|FireGridResolution/GenerationOptions|GetChunkFraction))
  (bind _returnvalue_2 (* _gridresolution _gridresolution_2))
  (bind _returnvalue_3 (/ _returnvalue_2 _chunkfraction))
  (bind _outactors (Actor|GetAllActorsOfClass "/Game/Packs_FX/ImpromptuFire/Blueprint/BP_FireSettingsVolume.BP_FireSettingsVolume_C"))
  (Variables|Default|SetFireSettingsVolumes _outactors) ; Get an array of fire settings volumes so we can use them later
  (if (Variables|FireGrid|GetAutoGenerate)
    (if (Variables|FireGrid|GetBuildGridUpwards)
      ;[1 1 1] Offset actor location going forward if we want to BuildGridUpwards
      (Transformation|SetActorLocation (+ (Transformation|GetActorLocation) (Math|Vector|MakeVector 0.0 0.0 (* (* (Variables|FireGridResolution/GenerationOptions|GetVerticalResolution) (* (Variables|FireGridResolution/GenerationOptions|GetCellHalfSize) 2.0)) 0.5))) false false)
      (Variables|FireGrid|SetIgnitionPoint (- (Variables|FireGrid|GetIgnitionPoint) (Math|Vector|MakeVector 0.0 0.0 (* (* (Variables|FireGridResolution/GenerationOptions|GetVerticalResolution) (* (Variables|FireGridResolution/GenerationOptions|GetCellHalfSize) 2.0)) 0.5)))))
    (Utilities|FlowControl|Delay (Variables|FireGrid|GetDelayBeforeStart))
    ;[1 1 1] Get Wind actor
    (bind _outactors_2 (Actor|GetAllActorsOfClass "/Script/Engine.WindDirectionalSource"))
    (Variables|Default|SetWind (Utilities|Array|Get(acopy) _outactors_2))
    ;[1 1 1] Set first cell location
    (Variables|Default|SetCellLocVec (Transformation|GetActorLocation))
    ;[1 1 1] Auto-light the grid
    (if (Variables|FireGrid|GetLight%20Automatically) ; Auto light?
      (Game|SpawnActorfromClass "/Game/Packs_FX/ImpromptuFire/Blueprint/BP_Flame.BP_Flame_C" (Math|Transform|MakeTransform (Math|Transform|TransformLocation (Transformation|GetActorTransform) (Variables|FireGrid|GetIgnitionPoint)) "0, 0, 0" "1.000000,1.000000,1.000000") "AlwaysSpawn" 0 0 true))
    (for _index (range 1 _returnvalue_3) :!label _label ; Loop through checking spaces for viable cell placement, placing cells. Cycle back into this loop with new locations for each grid chunk. We can delay between loops even though this is a regular for loop because the delay is outside the loop.
      (Variables|Default|SetCurrentCellIndex (+ _index (* (Variables|Default|GetChunksDone) _returnvalue_3)))
      (bind _overlapped (CallFunction|OverlapCheck (- (Math|Transform|InverseTransformLocation (Transformation|GetActorTransform) (Variables|Default|GetCellLocVec)) (Math|Vector|MakeVector (- (* (* (Variables|FireGridResolution/GenerationOptions|GetGridResolution) (* (Variables|FireGridResolution/GenerationOptions|GetCellHalfSize) 2.0)) 0.5) (Variables|FireGridResolution/GenerationOptions|GetCellHalfSize)) (- (* (* (Variables|FireGridResolution/GenerationOptions|GetGridResolution) (* (Variables|FireGridResolution/GenerationOptions|GetCellHalfSize) 2.0)) 0.5) (Variables|FireGridResolution/GenerationOptions|GetCellHalfSize)) (- (* (* (Variables|FireGridResolution/GenerationOptions|GetGridResolution) (* (Variables|FireGridResolution/GenerationOptions|GetCellHalfSize) 2.0)) 0.5) (Variables|FireGridResolution/GenerationOptions|GetCellHalfSize)))) false)) ; Check whether space is valid for a cell. Only make one if so
      (if _overlapped
        (bind _overlappedcell (CallFunction|OverlapCheck (- (Math|Transform|InverseTransformLocation (Transformation|GetActorTransform) (Variables|Default|GetCellLocVec)) (Math|Vector|MakeVector (- (* (* (Variables|FireGridResolution/GenerationOptions|GetGridResolution) (* (Variables|FireGridResolution/GenerationOptions|GetCellHalfSize) 2.0)) 0.5) (Variables|FireGridResolution/GenerationOptions|GetCellHalfSize)) (- (* (* (Variables|FireGridResolution/GenerationOptions|GetGridResolution) (* (Variables|FireGridResolution/GenerationOptions|GetCellHalfSize) 2.0)) 0.5) (Variables|FireGridResolution/GenerationOptions|GetCellHalfSize)) (- (* (* (Variables|FireGridResolution/GenerationOptions|GetGridResolution) (* (Variables|FireGridResolution/GenerationOptions|GetCellHalfSize) 2.0)) 0.5) (Variables|FireGridResolution/GenerationOptions|GetCellHalfSize)))) true)) ; Overlap check again, this time checking only for existing cells (any grid)
        (if _overlappedcell
          (if (== (Math|Integer|%(Integer) (Variables|Default|GetCurrentCellIndex) (/ (* _gridresolution_3 _gridresolution_3) (Variables|FireGridResolution/GenerationOptions|GetGridResolution))) 0) :!label _label_2 ; Begin a new row?
            (Variables|Default|SetCellLocVec (Math|Vector|MakeVector (.x (Transformation|GetActorLocation)) (+ (.y (Variables|Default|GetCellLocVec)) (* (Variables|FireGridResolution/GenerationOptions|GetCellHalfSize) 2.0)) (.z (Variables|Default|GetCellLocVec))))
            (else
              (Variables|Default|SetCellLocVec (Math|Vector|MakeVector (+ (.x (Variables|Default|GetCellLocVec)) (* (Variables|FireGridResolution/GenerationOptions|GetCellHalfSize) 2.0)) (.y (Variables|Default|GetCellLocVec)) (.z (Variables|Default|GetCellLocVec))))))
          (else
            (bind _returnvalue_4 (AddComponent|AddChildActorComponent false (Math|Transform|MakeTransform (- (Math|Transform|InverseTransformLocation (Transformation|GetActorTransform) (Variables|Default|GetCellLocVec)) (Math|Vector|MakeVector (- (* (* (Variables|FireGridResolution/GenerationOptions|GetGridResolution) (* (Variables|FireGridResolution/GenerationOptions|GetCellHalfSize) 2.0)) 0.5) (Variables|FireGridResolution/GenerationOptions|GetCellHalfSize)) (- (* (* (Variables|FireGridResolution/GenerationOptions|GetGridResolution) (* (Variables|FireGridResolution/GenerationOptions|GetCellHalfSize) 2.0)) 0.5) (Variables|FireGridResolution/GenerationOptions|GetCellHalfSize)) (- (* (* (Variables|FireGridResolution/GenerationOptions|GetGridResolution) (* (Variables|FireGridResolution/GenerationOptions|GetCellHalfSize) 2.0)) 0.5) (Variables|FireGridResolution/GenerationOptions|GetCellHalfSize))))))) ; Make a fire cell
            (bind _asbp_fire_cell (Utilities|Casting|CastToBP_FireCell (Variables|/Script/Engine.ChildActorComponent|GetChildActor _returnvalue_4)))
            (bind _returnvalue_5 (Utilities|Array|Add (Variables|Default|GetCells) _asbp_fire_cell))
            (Variables|/Game/Packs_FX/ImpromptuFire/Blueprint/BP_FireCell.BP_FireCell_C|SetIndexOnOwningGrid _asbp_fire_cell _returnvalue_5)
            (Variables|/Game/Packs_FX/ImpromptuFire/Blueprint/BP_FireCell.BP_FireCell_C|SetOwningGrid _asbp_fire_cell self)
            (Variables|/Game/Packs_FX/ImpromptuFire/Blueprint/BP_FireCell.BP_FireCell_C|SetCellHalfSize _asbp_fire_cell (Variables|FireGridResolution/GenerationOptions|GetCellHalfSize))
            (Default|CreateCell _asbp_fire_cell)
            (if (Variables|FireGrid|GetGridVisible)
              (Development|SetHiddeninGame _asbp_fire_cell false false) ; Unhide cells
              (goto _label_2))))
        (else
          (goto _label_2))))
    ;[1 1 1] Cycle back into the ForLoop for each chunk of grid, after a delay (only so we don't try to build the whole grid on one tick).
    (Variables|Default|SetChunksDone (+ (Variables|Default|GetChunksDone) 1))
    (if (>= (Variables|Default|GetChunksDone) _chunkfraction)
      (Utilities|FlowControl|Delay _gridloopdelay)
      ;[1 1 1] Keep doing all of the above as long as there's vertical iterations remaining
      (Variables|Default|SetVerticalIterations (+ (Variables|Default|GetVerticalIterations) 1))
      (if (>= (Variables|Default|GetVerticalIterations) (Variables|FireGridResolution/GenerationOptions|GetVerticalResolution))
        (Variables|Default|SetGridFullyGenerated true)
        ;[1 1 1] If no cells were generated, destroy this grid
        (if (== (Utilities|Array|Length (Variables|Default|GetCells)) 0)
          (Actor|DestroyActor))
        (else
          ;[1 1 1] finished all rows for this height, increment new cell height
          (Variables|Default|SetCellLocVec (Math|Vector|MakeVector (.x _returnvalue) (.y _returnvalue) (+ (.z _returnvalue) (* (Variables|Default|GetVerticalIterations) (* (Variables|FireGridResolution/GenerationOptions|GetCellHalfSize) 2.0)))))
          (Variables|Default|SetChunksDone 0)
          (goto _label)))
      (else
        (Utilities|FlowControl|Delay _gridloopdelay)
        (goto _label)))))

(fn ConstructionScript
  (bind _gridresolution (Variables|FireGridResolution/GenerationOptions|GetGridResolution))
  (bind _cellhalfsize (Variables|FireGridResolution/GenerationOptions|GetCellHalfSize))
  (bind _returnvalue (Math|Conversions|ToFloat(Integer) _gridresolution))
  (bind _returnvalue_2 (* _cellhalfsize 1.0))
  (bind _returnvalue_3 (* _returnvalue_2 _returnvalue))
  (bind _returnvalue_4 (AddComponent|AddBoxComponent false))
  (Components|Box|SetBoxExtent _returnvalue_4 (Math|Vector|MakeVector _returnvalue_3 _returnvalue_3 _returnvalue_3) false))

(fn OverlapCheck
  (params (CellPoint :type Vector) (CheckingForCells :type Boolean))
  (bind _returnvalue (Transformation|GetActorTransform))
  (bind _cellhalfsize (Variables|FireGridResolution/GenerationOptions|GetCellHalfSize))
  (bind _returnvalue_2 (Math|Transform|TransformLocation _returnvalue CellPoint))
  (bind _returnvalue_3 (* _cellhalfsize 1.0))
  (bind _returnvalue_4 (* _cellhalfsize 0.5))
  (if CheckingForCells
    ;[1 1 1] Check for overlaps with other cells - if there are any, we don't want a cell here
    (bind _returnvalue_5 (Collision|BoxOverlapActors _returnvalue_2 (Math|Vector|MakeVector _returnvalue_4 _returnvalue_4 _returnvalue_4) (Utilities|Array|MakeArray "ObjectTypeQuery2") "/Game/Packs_FX/ImpromptuFire/Blueprint/BP_FireCell.BP_FireCell_C" :!class /Script/Engine.KismetSystemLibrary))
    (else
      ;[1 1 1] Check for overlaps with worldstatic, ignoring cells. We only want to spawn cells where there's surface to burn
      (bind (_outhit _returnvalue_6) (Class|KismetSystemLibrary|BoxTraceSingleforObjects _returnvalue_2 (- _returnvalue_2 (Math|Vector|MakeVector 0.0 0.0 _returnvalue_4)) (Math|Vector|MakeVector _returnvalue_3 _returnvalue_3 _returnvalue_3) "0, 0, 0" (Utilities|Array|MakeArray "ObjectTypeQuery1") false (Variables|Default|GetCells) "None" true))))
  (return _returnvalue_6 _outhit _returnvalue_5))

(fn GetSettings
  (params (GridSettings :type BP%20Fire%20Grid%20Settings%20Structure))
  (Variables|FireGrid|SetIgnitionPoint (.ignitionpoint GridSettings))
  (Variables|FireGrid|SetMakeScorchDecals (.makescorchdecals GridSettings))
  (Variables|FireGrid|SetLight%20Automatically (.lightautomatically GridSettings))
  (Variables|FireGrid|SetBuildGridUpwards (.buildgridupwards GridSettings))
  (Variables|FireGrid|SetAllowCellCull (.allowcellcull GridSettings))
  (Variables|FireGrid|SetGridVisible (.gridvisible GridSettings))
  (Variables|FireGridResolution/GenerationOptions|SetCellHalfSize (.cellhalfsize GridSettings))
  (Variables|FireGridResolution/GenerationOptions|SetGridResolution (.gridresolution GridSettings))
  (Variables|FireGridResolution/GenerationOptions|SetVerticalResolution (.verticalresolution GridSettings))
  (Variables|FireGridResolution/GenerationOptions|SetChunkFraction (.chunkfraction GridSettings))
  (if (.autogenerate GridSettings)
    (CallFunction|Generate)))