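; Fire energy VFX Blueprint that plays an appearance effect on its Girl skeletal mesh at BeginPlay.
; Timeline_0 scrubs the mesh's animation position and drives the "Mask" material parameter, whose preliminary set to 1.0 is immediately overwritten each update.
; The timeline's Spawn event attaches the P_Appear emitter at an offset from Girl.
; The node passing Girl's owner as the emitter's VertSurfaceActor parameter is disconnected.
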(event EventBeginPlay
  (bind _girl (Variables|Default|Getgirl))
  (bind (_direction _mask _anim) (Timeline|Timeline_0 Play)
    (:Update
      (Components|Animation|SetPosition (Variables|Default|Getgirl) _anim true)
      (Rendering|Material|SetScalarParameterValueonMaterials _girl "Mask" 1.0)
      (Rendering|Material|SetScalarParameterValueonMaterials _girl "Mask" _mask))
    (:spawn
      (bind _returnvalue (Effects|SpawnEmitterAttached "/Game/Packs_FX/FireEnergyVFX/Particles/P_Appear.P_Appear" _girl "None" (+ (Transformation|GetWorldLocation _girl) "0,-200.000000,200.000000") "0, 0, 0" "1.000000,1.000000,1.000000" "KeepWorldPosition")))))

(fn ConstructionScript)