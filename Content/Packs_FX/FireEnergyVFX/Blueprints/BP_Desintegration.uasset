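; BP_Desintegration is a demo Blueprint from the Fire Energy VFX pack that plays a disintegration effect on the Girl mesh.
; On BeginPlay, a timeline scrubs the mesh's animation position and drives a "Mask" scalar parameter on its materials.
; A timeline event spawns the P_CharSmoke emitter attached to the mesh, passing its owning actor as the VertSurfaceActor parameter for particle sourcing.
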(event EventBeginPlay
  (bind _girl (Variables|Default|Getgirl))
  (bind (_direction _mask _anim) (Timeline|Timeline_0 Play)
    (:Update
      (Components|Animation|SetPosition (Variables|Default|Getgirl) _anim true)
      (Rendering|Material|SetScalarParameterValueonMaterials _girl "Mask" _mask))
    (:spawn
      (bind _returnvalue (Effects|SpawnEmitterAttached "/Game/Packs_FX/FireEnergyVFX/Particles/P_CharSmoke.P_CharSmoke" _girl "None" (Transformation|GetWorldLocation _girl) "0, 0, 0" "1.000000,1.000000,1.000000" "KeepWorldPosition"))
      (Variables|/Script/Engine.ParticleSystemComponent|SetInstanceParameters _returnvalue (Utilities|Array|MakeArray (Utilities|Struct|MakeParticleSysParam "VertSurfaceActor" "PSPT_Actor" 0.0 0.0 "0.000000,0.000000,0.000000" "0.000000,0.000000,0.000000" "(B=0,G=0,R=0,A=0)" (Components|GetOwner (Variables|Default|Getgirl))))))))

(fn ConstructionScript)