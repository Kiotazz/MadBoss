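; Explosive barrel actor that ignites when fire damage depletes its HP, or on BeginPlay if set to auto-ignite.
; Ignition plays sparks for a random fuse time, then spawns the explosion effect and sound.
; A sphere overlap sends ignite messages through the fire interface and pushes static mesh actors and other barrels with radial force.
; Optionally, a downward sphere trace places a spreading fire grid at the blast site.
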(event EventBeginPlay
  ;[1 1 1] Auto-ignite
  (if (Variables|Barrel|GetAutoIgnite)
    (CallFunction|Ignite)))

(event EventFireDamage
  (params (Amount :type Integer))
  ;[1 1 1] Recieve fire damage and trigger ignition
  (Variables|Barrel|SetHP (- (Variables|Barrel|GetHP) Amount))
  (if (<= (Variables|Barrel|GetHP) 0)
    (Utilities|FlowControl|DoOnce false
      (:Completed
        (CallFunction|Ignite)))))

(event EventIgnite
  (bind _barrel (Variables|Default|GetBarrel))
  (bind _barrel_2 (Variables|Default|GetBarrel))
  (bind _returnvalue (Transformation|GetWorldLocation _barrel))
  (bind _returnvalue_2 (Transformation|GetWorldLocation _barrel_2))
  ;[1 1 1] Ignite, explode, build and light fire grid
  (Variables|Barrel|SetAlight true)
  (bind _returnvalue_3 (AddComponent|AddParticleSystemComponent self false (Math|Transform|MakeTransform "0, 0,30.000000" "0, 0, 0" "1,1,1")))
  (Transformation|SetRelativeScale3D _returnvalue_3 "2.000000,2.000000,30.000000")
  (bind _returnvalue_4 (Audio|SpawnSoundAttached "/Game/Packs_FX/ImpromptuFire/StarterContent/Audio/Fire_Sparks01_Cue.Fire_Sparks01_Cue" (Variables|Default|GetBarrel) "None" "0, 0, 0" "0, 0, 0" "KeepRelativeOffset" true 1.0 1.0 0.0 0 0))
  (Utilities|FlowControl|Delay (Math|Random|RandomFloatinRange (Variables|Barrel|GetMinFuseTime) (Variables|Barrel|GetMaxFuseTime)))
  (bind _returnvalue_5 (Effects|SpawnEmitteratLocation "/Game/Packs_FX/ImpromptuFire/StarterContent/Particles/P_Explosion.P_Explosion" (Transformation|GetWorldLocation)))
  (Transformation|SetRelativeScale3D _returnvalue_5 "3.000000,3.000000,3.000000")
  (Audio|Components|Audio|Stop _returnvalue_4)
  (Components|DestroyComponent _returnvalue_4)
  (Audio|SpawnSoundAttached "/Game/Packs_FX/ImpromptuFire/StarterContent/Audio/Explosion_Cue.Explosion_Cue" _barrel_2 "None" "0, 0, 0" "0, 0, 0" "KeepRelativeOffset" false 2.0 1.0 0.0 0 0)
  (bind _outactors (Collision|SphereOverlapActors _returnvalue_2 512.0 (Utilities|Array|MakeArray "ObjectTypeQuery4") 0))
  (for _array_element _outactors
    (if (Utilities|DoesObjectImplementInterface _array_element "/Game/Packs_FX/ImpromptuFire/Blueprint/BP_FireInterface.BP_FireInterface_C")
      (Class|BPFireInterface|Ignite(Message) _array_element))
    (bind _as静态网格体actor (Utilities|Casting|CastToStaticMeshActor _array_element)
      (:then
        _)
      (:CastFailed
        (bind _asbp_explosive_barrel (Utilities|Casting|CastToBP_ExplosiveBarrel _array_element))))
    (Physics|AddRadialForce (Variables|/Script/Engine.StaticMeshActor|GetStaticMeshComponent _as静态网格体actor) _returnvalue_2 512.0 2e+07 "RIF_Constant" false 0))
  (if (Variables|Barrel|GetStartFireOnExplode)
    (bind (_outhit _returnvalue_6) (Collision|SphereTraceForObjects _returnvalue (- _returnvalue "0, 0,5.000000") 2e+02 (Utilities|Array|MakeArray "ObjectTypeQuery1") false 0 "None"))
    (if _returnvalue_6
      (Utilities|Struct|SetmembersinBP_FireGridSettings (Variables|Barrel|GetExplosionFireGrid) (Math|Transform|InverseTransformLocation (Math|Transform|MakeTransform _returnvalue "0, 0, 0" "1,1,1") _returnvalue)) ; Override IgnitionPoint
      (Utilities|MakeFireGrid (Variables|Barrel|GetExplosionFireGrid) (.Location (Collision|BreakHitResult _outhit))
        (:Out
          _)))
    (Actor|DestroyActor)))

(fn ConstructionScript)