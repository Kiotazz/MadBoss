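; Projectile that spreads fire by creating auto-igniting, upward-building fire grids where it hits non-physics surfaces.
; Hits on simulating bodies apply a velocity-scaled impulse instead of spawning a grid.
; A DoOnce, reset by a Tick-driven Delay of NewGridInterval, keeps rapid bounces from creating many grids.
; It sends fire damage through BP_FireInterface to actors it hits and to those in a small sphere overlap every tick.
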(event EventTick
  (params (DeltaSeconds :type Float%20%28single-precision%29))
  ;[1 1 1] Deal fire damage in a range
  (Utilities|FlowControl|Sequence
    (:then_0
      (bind (_outactors _returnvalue) (Collision|SphereOverlapActors (Transformation|GetActorLocation) 32.0 (Utilities|Array|MakeArray "ObjectTypeQuery2" "ObjectTypeQuery1") 0))
      (if _returnvalue
        (for _array_element _outactors
          (if (Utilities|DoesObjectImplementInterface _array_element "/Game/Packs_FX/ImpromptuFire/Blueprint/BP_FireInterface.BP_FireInterface_C")
            (Class|BPFireInterface|FireDamage(Message) _array_element 50)))))
    (:then_1
      (Utilities|FlowControl|Delay (Variables|Default|GetNewGridInterval))
      (Utilities|FlowControl|DoOnce false) ; enters at Reset
    )))

(event Collision|EventHit
  (params (MyComp :type Primitive%20Component%20Object%20Reference) (Other :type Actor%20Object%20Reference) (OtherComp :type Primitive%20Component%20Object%20Reference) (bSelfMoved :type Boolean) (HitLocation :type Vector :default "0, 0, 0") (HitNormal :type Vector :default "0, 0, 0") (NormalImpulse :type Vector :default "0, 0, 0") (Hit :type Hit%20Result%20Structure%20%28by%20ref%29))
  (Utilities|FlowControl|Sequence
    (:then_0
      (if (Physics|IsSimulatingPhysics OtherComp "None")
        (Physics|AddImpulseatLocation OtherComp (* (Transformation|GetVelocity) 1e+02) (Transformation|GetActorLocation) "None") ; Apply impulse to physics objects
        (else
          (Utilities|FlowControl|DoOnce false ; Reset every NewGridInterval so rapid bouncing doesn't result in many many grids
            (:Completed
              (Utilities|MakeFireGrid (Utilities|Struct|MakeBP_FireGridSettings true (Math|Transform|InverseTransformLocation (Math|Transform|MakeTransform HitLocation) HitLocation) true true true true false 64.0 8 8 8 0.0) HitLocation) ; Make auto-igniting fire grid
            )))))
    (:then_1
      (if (Utilities|DoesObjectImplementInterface Other "/Game/Packs_FX/ImpromptuFire/Blueprint/BP_FireInterface.BP_FireInterface_C")
        (Class|BPFireInterface|FireDamage(Message) Other 50) ; Deal fire damage on hit
      ))))

(fn ConstructionScript)