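; VR effect Blueprint that repeatedly fires electric arcs between its Start and End components.
; Tick feeds a Delay of random length scaled by Frequency, so it acts as a repeating timer.
; Each firing spawns an auto-destroying Niagara arc system attached to Start, passing End's world location as the target.
; Randomized decline flag, ribbon width, brightness boost and blue-leaning color vary each arc, while reversal stays off.
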(event EventTick
  (params (DeltaSeconds :type Float%20%28single-precision%29))
  ;[1 1 1] Frequency
  (Utilities|FlowControl|Delay (* (Math|Random|RandomFloatinRange 1.0 3.0) (Variables|Default|GetFrequency)))
  ;[1 1 1] Add lightning effect
  (bind _returnvalue (Niagara|SpawnSystemAttached "/Game/Packs_FX/Lightning_Electricity_Pack/Virtual_Reality/VR_Particles/P_VR_ArcsBetween2points.P_VR_ArcsBetween2points" (Variables|Default|GetStart) "None" "0, 0, 0" "0, 0, 0" "KeepRelativeOffset" true))
  (Effects|Components|ParticleSystem|SetVectorParameter _returnvalue "User.End" (Transformation|GetWorldLocation (Variables|Default|GetEnd)))
  (Class|NiagaraComponent|SetVariableBool _returnvalue "User.ArcDeclining" (Math|Random|RandomBool))
  (Class|NiagaraComponent|SetVariableBool _returnvalue "User.ArcReverse" false)
  (Effects|Components|ParticleSystem|SetFloatParameter _returnvalue "User.RibbonWidth" (Math|Random|RandomFloatinRange 1.5 2.5))
  (Effects|Components|ParticleSystem|SetFloatParameter _returnvalue "User.ColorBoost" (Math|Random|RandomFloatinRange 3e+01 7e+01))
  (Effects|Components|ParticleSystem|SetColorParameter _returnvalue "User.Color" (Utilities|Struct|MakeLinearColor (Math|Random|RandomFloatinRange 0.0 0.4) (Math|Random|RandomFloatinRange 0.25 0.6) (Math|Random|RandomFloatinRange 0.6 1.0) 1.0)))

(fn ConstructionScript)