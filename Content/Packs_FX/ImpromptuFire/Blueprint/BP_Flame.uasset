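; BP_Flame is a fire actor that periodically damages nearby objects and can burn out after a set lifetime.
; A Delay on Tick paces a sphere overlap on world and physics object types, sending fire damage to hits implementing BP_FireInterface.
; On BeginPlay, a non-zero Lifetime schedules deactivation of the Fire component, then actor destruction after a short grace delay.
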(event EventBeginPlay
  (if (not (== (Variables|Default|GetLifetime) 0.0))
    (Utilities|FlowControl|Delay (Variables|Default|GetLifetime))
    (Components|Activation|Deactivate (Variables|Default|GetFire))
    (Utilities|FlowControl|Delay 4.0)
    (Actor|DestroyActor)))

(event EventTick
  (params (DeltaSeconds :type Float%20%28single-precision%29))
  (Utilities|FlowControl|Delay (Variables|Default|GetFireDamageInterval))
  (bind (_outactors _returnvalue) (Collision|SphereOverlapActors (Transformation|GetActorLocation) (Variables|Default|GetFireDamageRadius) (Utilities|Array|MakeArray "ObjectTypeQuery2" "ObjectTypeQuery1" "ObjectTypeQuery4") 0))
  (if _returnvalue
    (for _array_element _outactors
      (if (Utilities|DoesObjectImplementInterface _array_element "/Game/Packs_FX/ImpromptuFire/Blueprint/BP_FireInterface.BP_FireInterface_C")
        (Class|BPFireInterface|FireDamage(Message) _array_element (Variables|Default|GetFireDamagePerInterval))))))

(fn ConstructionScript)